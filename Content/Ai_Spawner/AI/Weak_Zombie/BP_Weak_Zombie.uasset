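; Weak zombie enemy Blueprint that chases the player with randomized health and walk speed, attacking on arrival.
; A looping timer reissues AI MoveTo; arrival triggers a punch or crawl bite, while hitbox overlap applies cooldown-gated damage.
; Taking damage spawns blood and can randomly trigger a faster, harder-hitting run.
; At zero health it randomly either starts crawling or ragdolls, pays the player and is destroyed, as it does on ReceiveBarrel.
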(event OnComponentBeginOverlap(Hitbox)
  (params (OverlappedComponent :type Primitive%20Component%20Object%20Reference) (OtherActor :type Actor%20Object%20Reference) (OtherComp :type Primitive%20Component%20Object%20Reference) (OtherBodyIndex :type Integer) (bFromSweep :type Boolean) (SweepResult :type Hit%20Result%20Structure%20%28by%20ref%29))
  ;[1 1 1] Damage to player
  (bind _asplayer (Utilities|Casting|CastToPlayer OtherActor))
  (if (Variables|Default|GetRun)
    (Utilities|FlowControl|DoOnce false :!label _label
      (:Completed
        (Game|Damage|ApplyDamage _asplayer (Variables|Default|GetExtraDamage) 0 0)
        (Utilities|FlowControl|Delay 1.9)
        (goto _label Reset)))
    (else
      (Utilities|FlowControl|DoOnce false :!label _label_2
        (:Completed
          (Game|Damage|ApplyDamage _asplayer (Variables|Default|GetDamage) 0 0)
          (Utilities|FlowControl|Delay 3.8)
          (goto _label_2 Reset))))))

(event Custom|MoveToPlayer
  (bind _returnvalue (Game|GetPlayerCharacter 0))
  (bind _self self)
  (bind _charactermovement (Variables|Character|GetCharacterMovement))
  (AI|AIMoveTo _self "0, 0, 0" _returnvalue 1e+01 false
    (:OnSuccess
      (Utilities|FlowControl|DoOnce false :!label _label
        (:Completed
          (if (Variables|Default|GetCrawl)
            (Transformation|SetActorRelativeRotation (Math|Rotator|FindLookatRotation (Math|Vector|GetForwardVector (Variables|Character|GetMesh)) (Transformation|GetActorLocation (Game|GetPlayerCharacter 0))) false true)
            (Utilities|FlowControl|DoOnce false :!label _label_2
              (:Completed
                (Variables|Default|SetCrawlBite true)
                (Variables|/Script/Engine.CharacterMovementComponent|SetMaxWalkSpeed _charactermovement 0.0)
                (Utilities|FlowControl|Delay 1.5)
                (Variables|Default|SetCrawlBite false)
                (Variables|/Script/Engine.CharacterMovementComponent|SetMaxWalkSpeed _charactermovement (Math|Random|RandomFloatinRange 5e+01 1e+02))
                (Variables|Default|SetCrawl true)
                (goto _label_2 Reset)))
            (else
              (Utilities|FlowControl|DoOnce false :!label _label_3
                (:Completed
                  (Components|Activation|SetActive (Variables|Default|GetHitbox) true false)
                  (Variables|Default|SetPunch true))))))))
    (:OnFail
      (Utilities|FlowControl|Sequence
        (:then_0
          (goto _label Reset))
        (:then_1
          (AI|AIMoveTo _self "0, 0, 0" _returnvalue 1e+01 false))
        (:then_2
          (Variables|Default|SetPunch false)
          (Components|Activation|SetActive (Variables|Default|GetHitbox) true false)
          (goto _label_3 Reset))))))

(event Custom|ReceiveBarrel
  ;[1 1 1] Death & Crawl // Die physic
  (Physics|SetSimulatePhysics (Variables|Character|GetMesh) true)
  (Collision|SetCollisionEnabled (Variables|Collision|GetCapsuleComponent) "NoCollision")
  (bind _asplayer (Utilities|Casting|CastToPlayer (Game|GetPlayerCharacter 0)))
  (Variables|/Game/Player/Blueprints/Player.Player_C|SetMoney _asplayer (+ (Variables|Default|GetPrice) (Variables|/Game/Player/Blueprints/Player.Player_C|GetMoney _asplayer)))
  (Utilities|FlowControl|Delay 1.0)
  (Actor|DestroyActor))

(event Custom|Explosion
  ;[1 1 1] Death & Crawl // Die physic
  (switch int (Math|Random|RandomIntegerinRange 0 10)
    (:0
      (Physics|SetSimulatePhysics (Variables|Character|GetMesh) true :!label _label)
      (Collision|SetCollisionEnabled (Variables|Collision|GetCapsuleComponent) "NoCollision")
      (bind _asplayer (Utilities|Casting|CastToPlayer (Game|GetPlayerCharacter 0)))
      (Variables|/Game/Player/Blueprints/Player.Player_C|SetMoney _asplayer (+ (Variables|Default|GetPrice) (Variables|/Game/Player/Blueprints/Player.Player_C|GetMoney _asplayer)))
      (Utilities|FlowControl|Delay 1.0)
      (Actor|DestroyActor))
    (:1
      (goto _label))
    (:2
      (goto _label))
    (:3
      (goto _label))
    (:4
      (goto _label))
    (:5
      (goto _label))
    (:6
      (goto _label))
    (:7
      (goto _label))
    (:8
      (Variables|Default|SetCrawl true :!label _label_2))
    (:9
      (goto _label_2))
    (:10
      (goto _label_2))))

(event EventBeginPlay
  (Utilities|FlowControl|Sequence
    (:then_0
      (Components|Activation|SetActive (Variables|Default|GetHitbox) false false))
    (:then_1
      (Variables|/Script/Engine.CharacterMovementComponent|SetMaxWalkSpeed (Variables|Character|GetCharacterMovement) (Math|Random|RandomFloatinRange 5e+01 1e+02)))
    (:then_2
      (Utilities|Time|SetTimerbyEvent (delegate Custom|MoveToPlayer) 0.05 true)
      (CallFunction|MovetoPlayer))
    (:then_3
      (bind _output_get (Variables|Default|SetHealth (Math|Random|RandomFloatinRange 5e+01 2e+02)))
      (Variables|Default|SetMaxHealth _output_get))))

(event Game|Damage|EventAnyDamage
  (params (Damage :type Float%20%28single-precision%29) (DamageType :type Damage%20Type%20Object%20Reference) (InstigatedBy :type Controller%20Object%20Reference) (DamageCauser :type Actor%20Object%20Reference))
  ;[1 1 1] Death & Crawl // Die physic
  (Variables|Default|SetHealth (- (Variables|Default|GetHealth) Damage))
  (Effects|SpawnEmitterAttached "/Game/Polygon_BattleRoyale/ParticleFX/FX_Blood.FX_Blood" (Variables|Character|GetMesh) "None" "0, 0, 0" "0, 0, 0" "2.000000,2.000000,2.000000")
  (Utilities|FlowControl|Sequence
    (:then_0
      (if (<= (Variables|Default|GetHealth) 0.0)
        (switch int (Math|Random|RandomIntegerinRange 0 10)
          (:0
            (Physics|SetSimulatePhysics (Variables|Character|GetMesh) true :!label _label)
            (Collision|SetCollisionEnabled (Variables|Collision|GetCapsuleComponent) "NoCollision")
            (bind _asplayer (Utilities|Casting|CastToPlayer (Game|GetPlayerCharacter 0)))
            (Variables|/Game/Player/Blueprints/Player.Player_C|SetMoney _asplayer (+ (Variables|Default|GetPrice) (Variables|/Game/Player/Blueprints/Player.Player_C|GetMoney _asplayer)))
            (Utilities|FlowControl|Delay 1.0)
            (Actor|DestroyActor))
          (:1
            (goto _label))
          (:2
            (goto _label))
          (:3
            (goto _label))
          (:4
            (goto _label))
          (:5
            (goto _label))
          (:6
            (goto _label))
          (:7
            (goto _label))
          (:8
            (Variables|Default|SetCrawl true :!label _label_2))
          (:9
            (goto _label_2))
          (:10
            (goto _label_2)))))
    (:then_1
      (if (< (Math|Float|%(Float) (Variables|Default|GetHealth) 5e+01) (Variables|Default|GetMaxHealth))
        (switch int (Math|Random|RandomIntegerinRange 0 5)
          (:3
            _)
          (:7
            _))
        (Variables|Default|SetRun true)
        (Variables|/Script/Engine.CharacterMovementComponent|SetMaxWalkSpeed (Variables|Character|GetCharacterMovement) 3e+02)))))

(fn ConstructionScript)