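; Explosive barrel interactable that explodes when shot and is coded to double as generator fuel.
; Pistol, shotgun or LMG bullets entering the Box trigger a one-shot explosion with radial impulse, damage, camera shake and FX, then delayed destruction.
; Sphere overlap holds branches for refueling an Electric_Generator and for ragdolling a weak zombie on a fast hit, both gated behind a Player cast of the same overlapping actor.
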(event OnComponentBeginOverlap(Sphere)
  (params (OverlappedComponent :type Primitive%20Component%20Object%20Reference) (OtherActor :type Actor%20Object%20Reference) (OtherComp :type Primitive%20Component%20Object%20Reference) (OtherBodyIndex :type Integer) (bFromSweep :type Boolean) (SweepResult :type Hit%20Result%20Structure%20%28by%20ref%29))
  (bind _asplayer (Utilities|Casting|CastToPlayer OtherActor))
  (Utilities|FlowControl|Sequence
    (:then_0
      (bind _aselectric_generator (Utilities|Casting|CastToElectric_Generator OtherActor))
      (Variables|/Game/GPE/Assets_Interaction/Electric_Generator.Electric_Generator_C|SetFuel_Capacity _aselectric_generator (+ (Variables|Default|GetFuel_Ammount) (Variables|/Game/GPE/Assets_Interaction/Electric_Generator.Electric_Generator_C|GetFuel_Capacity _aselectric_generator)))
      (Variables|/Game/Player/Blueprints/Player.Player_C|SetIsHoldingObject? _asplayer false)
      (Default|ShowPreviewBarrel _aselectric_generator)
      (Actor|DestroyActor))
    (:then_1
      (bind _asbp_weak_zombie (Utilities|Casting|CastToBP_Weak_Zombie OtherActor))
      (if (> (Math|Vector|VectorLength (Transformation|GetComponentVelocity (Variables|Default|GetStaticMesh))) 5e+01)
        (Utilities|FlowControl|Sequence
          (:then_0
            (Class|RadialForceComponent|FireImpulse (Variables|Default|GetRadialForce))
            (Physics|SetSimulatePhysics (Variables|/Script/Engine.Character|GetMesh _asbp_weak_zombie) true)
            (Actor|DestroyActor))
          (:then_1
            (Utilities|FlowControl|DoOnce false
              (:Completed
                (bind _returnvalue (Effects|SpawnEmitterAttached "/Game/Polygon_BattleRoyale/ParticleFX/FX_Explosion.FX_Explosion" (Variables|Default|GetStaticMesh) "None" "0, 0, 0" "0, 0, 0" "1.000000,1.000000,1.000000" "SnapToTargetIncludingScale"))
                (Utilities|FlowControl|Delay 2.5)
                (Components|DestroyComponent _returnvalue)))))))))

(event OnComponentBeginOverlap(Box)
  (params (OverlappedComponent :type Primitive%20Component%20Object%20Reference) (OtherActor :type Actor%20Object%20Reference) (OtherComp :type Primitive%20Component%20Object%20Reference) (OtherBodyIndex :type Integer) (bFromSweep :type Boolean) (SweepResult :type Hit%20Result%20Structure%20%28by%20ref%29))
  (Utilities|FlowControl|Sequence
    (:then_0
      (Utilities|Casting|CastToPistol_Bullet OtherActor))
    (:then_1
      (Utilities|Casting|CastToShotgun_Bullet OtherActor))
    (:then_2
      (Utilities|Casting|CastToLMG_Bullet OtherActor)))
  (CallFunction|Explosion))

(event Custom|Explosion
  (Utilities|FlowControl|DoOnce false
    (:Completed
      (Variables|Default|SetExplosion? true)
      (Utilities|FlowControl|Sequence
        (:then_0
          (Class|RadialForceComponent|FireImpulse (Variables|Default|GetRadialForce))
          (Camera|PlayWorldCameraShake "/Game/Player/Blueprints/WeaponsCameraShake/ExplosiveBarrel_CameraShake.ExplosiveBarrel_CameraShake_C" (Transformation|GetWorldLocation (Variables|Default|GetRadialForce)) 0.0 3e+02 0.0 true)
          (Class|GameplayStatics|ApplyRadialDamagewithFalloff 5e+02 0.0 (Transformation|GetWorldLocation (Variables|Default|GetRadialForce)) 3e+02 4e+02 0.0 "/Script/Engine.DamageType" 0 0 0 "ECC_Visibility")
          (Components|DestroyComponent (Variables|Default|GetStaticMesh)))
        (:then_1
          (Utilities|FlowControl|DoOnce false
            (:Completed
              (bind _returnvalue (Effects|SpawnEmitterAttached "/Game/Polygon_BattleRoyale/ParticleFX/FX_Explosion.FX_Explosion" (Variables|Default|GetStaticMesh) "None" "0, 0, 0" "0, 0, 0" "1.000000,1.000000,1.000000" "SnapToTargetIncludingScale"))
              (Utilities|FlowControl|Delay 2.5)
              (Components|DestroyComponent _returnvalue))))
        (:then_2
          (Utilities|FlowControl|Delay 2.5)
          (Actor|DestroyActor))))))

(event Collision|EventActorBeginOverlap
  (params (OtherActor :type Actor%20Object%20Reference)))

(event EventTick
  (params (DeltaSeconds :type Float%20%28single-precision%29)))

(fn ConstructionScript)