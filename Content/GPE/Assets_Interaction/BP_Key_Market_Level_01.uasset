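; BP_Key_Market_Level_01 is an interactable key pickup for the Level 01 objective to search for the key.
; On Interaction, it sets HasKey on the Player character if not already set, then hides its mesh and disables that mesh's collision instead of destroying the actor.
; It then finds the W_Level01_Objectives widget by class and turns its Searchthekey entry green.
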(event EventBeginPlay)

(event Collision|EventActorBeginOverlap
  (params (OtherActor :type Actor%20Object%20Reference)))

(event EventTick
  (params (DeltaSeconds :type Float%20%28single-precision%29)))

(event EventInteraction
  (bind _staticmesh (Variables|Default|GetStaticMesh))
  ;[1 1 1] Take & Destroy key
  (bind _asplayer (Utilities|Casting|CastToPlayer (Game|GetPlayerCharacter 0)))
  (if (not (Variables|/Game/Player/Blueprints/Player.Player_C|GetHasKey? _asplayer))
    (Variables|/Game/Player/Blueprints/Player.Player_C|SetHasKey? _asplayer true)
    (Rendering|SetVisibility _staticmesh false false)
    (Collision|SetCollisionEnabled _staticmesh "NoCollision")
    (bind _foundwidgets (Widget|GetAllWidgetsOfClass "/Game/Widget/LevelObjective/W_Level01_Objectives.W_Level01_Objectives_C" true))
    (Appearance|SetColorandOpacity (Variables|/Game/Widget/LevelObjective/W_Level01_Objectives.W_Level01_Objectives_C|GetSearchthekey (Utilities|Array|Get(acopy) _foundwidgets)) (Utilities|Struct|MakeSlateColor "(R=0.000000,G=1.000000,B=0.000000,A=1.000000)") :!class /Script/UMG.TextBlock)))

(fn ConstructionScript)