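; BP_Lock is an interactable lock that destroys itself when the player interacts while holding a matching key.
; Its Interaction event casts player character 0 to Player and checks the HasKey flag.
; It then compares its own ID with that of the first BP_Key found in the level through GetAllActorsOfClass, rather than a key referenced by the player.
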(event EventBeginPlay)

(event Collision|EventActorBeginOverlap
  (params (OtherActor :type Actor%20Object%20Reference)))

(event EventTick
  (params (DeltaSeconds :type Float%20%28single-precision%29)))

(event EventInteraction
  (bind _asplayer (Utilities|Casting|CastToPlayer (Game|GetPlayerCharacter 0)))
  (if (Variables|/Game/Player/Blueprints/Player.Player_C|GetHasKey? _asplayer)
    (bind _outactors (Actor|GetAllActorsOfClass "/Game/GPE/Assets_Interaction/Bp_Key.BP_Key_C"))
    (if (== (Variables|/Game/GPE/Assets_Interaction/Bp_Key.BP_Key_C|GetID (Utilities|Array|Get(acopy) _outactors)) (Variables|Default|GetID))
      (Actor|DestroyActor))))

(fn ConstructionScript)