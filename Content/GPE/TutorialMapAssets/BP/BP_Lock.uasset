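; BP_Lock is a tutorial-map lock actor that is destroyed when interacted with by a player holding a key.
; Interaction checks the Player's HasKey flag, then compares its ID only against the first BP_Lock found in the level before destroying itself.
; A Sphere overlap by the Player creates a FindTheKey prompt widget, and any end overlap removes it without checking the actor.
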(event OnComponentBeginOverlap(Sphere)
  (params (OverlappedComponent :type Primitive%20Component%20Object%20Reference) (OtherActor :type Actor%20Object%20Reference) (OtherComp :type Primitive%20Component%20Object%20Reference) (OtherBodyIndex :type Integer) (bFromSweep :type Boolean) (SweepResult :type Hit%20Result%20Structure%20%28by%20ref%29))
  (Utilities|Casting|CastToPlayer OtherActor)
  (bind _returnvalue (UserInterface|CreateWidget "/Game/GPE/TutorialMapAssets/Widgets/FindTheKey.FindTheKey_C" (Game|GetPlayerController 0)))
  (bind _output_get (Variables|Default|SetW_FindTheKey _returnvalue))
  (UserInterface|Viewport|AddtoViewport _output_get 0))

(event OnComponentEndOverlap(Sphere)
  (params (OverlappedComponent :type Primitive%20Component%20Object%20Reference) (OtherActor :type Actor%20Object%20Reference) (OtherComp :type Primitive%20Component%20Object%20Reference) (OtherBodyIndex :type Integer))
  (Widget|RemovefromParent (Variables|Default|GetW_FindTheKey)))

(event EventBeginPlay)

(event Collision|EventActorBeginOverlap
  (params (OtherActor :type Actor%20Object%20Reference)))

(event EventTick
  (params (DeltaSeconds :type Float%20%28single-precision%29)))

(event EventInteraction
  (bind _asplayer (Utilities|Casting|CastToPlayer (Game|GetPlayerCharacter 0)))
  (if (Variables|/Game/Player/Blueprints/Player.Player_C|GetHasKey? _asplayer)
    (bind _outactors (Actor|GetAllActorsOfClass "BP_Lock_C"))
    (if (== (Variables|BP_Lock_C|GetID (Utilities|Array|Get(acopy) _outactors)) (Variables|Default|GetID))
      (Actor|DestroyActor))))

(fn ConstructionScript)