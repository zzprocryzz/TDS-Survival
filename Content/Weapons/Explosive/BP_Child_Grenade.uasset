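; Child grenade Blueprint that adds the explosion behavior to its parent class through a GrenadeGoesBoom event.
; After a short fuse delay, it fires the RadialForce impulse and destroys the skeletal mesh.
; It then attaches an explosion particle effect to the RadialForce component and removes that effect after a further delay.
; The actor itself is not destroyed here, and BeginPlay only calls the parent.
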(event Custom|GrenadeGoesBoom
  (Utilities|FlowControl|Delay 1.0)
  (Class|RadialForceComponent|FireImpulse (Variables|Default|GetRadialForce))
  (Utilities|FlowControl|Sequence
    (:then_0
      (Components|DestroyComponent (Variables|Default|GetSkeletalMesh)))
    (:then_1
      (bind _returnvalue (Effects|SpawnEmitterAttached "/Game/Polygon_BattleRoyale/ParticleFX/FX_Explosion.FX_Explosion" (Variables|Default|GetRadialForce) "None"))
      (Utilities|FlowControl|Delay 2.5)
      (Components|DestroyComponent _returnvalue))))

(event EventBeginPlay
  (|CallParentFunction))

(event Collision|EventActorBeginOverlap
  (params (OtherActor :type Actor%20Object%20Reference))
  (|CallParentFunction OtherActor) ; This node is disabled and will not be called.\nDrag off pins to build functionality.
)

(event EventTick
  (params (DeltaSeconds :type Float%20%28single-precision%29))
  (|CallParentFunction DeltaSeconds) ; This node is disabled and will not be called.\nDrag off pins to build functionality.
)

(fn ConstructionScript
  (|CallParentFunction))